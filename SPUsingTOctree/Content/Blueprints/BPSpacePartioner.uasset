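; Octree demo Blueprint that sets up a spatial partition at BeginPlay and populates it with a few randomly placed test actors.
; It initializes the octree over a fixed box centered on the origin, with optional debug drawing.
; A random stream drives how many OctreeDemoElement actors spawn and where within that box.
; Each spawned actor is registered as an octree element using the bounds of its Cube component.
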(event `self.ReceiveBeginPlay`
  (bind _randstream (`self.RandStream`))
  ;[1 1 1] Initialize Octree
  (`self.Initialize` (make `Box` (-1000.0 -1000.0 -1000.0) (1000.0 1000.0 1000.0)) (`self.DrawDebugInfo`))
  (for _ (range (+ (`KismetMathLibrary.RandomIntegerInRangeFromStream` 2 3 _randstream) 1))
    (bind _returnvalue (`|SpawnActorFromClass` "/Game/Blueprints/OctreeDemoElement.OctreeDemoElement_C" (`KismetMathLibrary.MakeTransform` (`KismetMathLibrary.MakeVector` (`KismetMathLibrary.RandomFloatInRangeFromStream` -1000.0 1000.0 _randstream) (`KismetMathLibrary.RandomFloatInRangeFromStream` -1000.0 1000.0 _randstream) (`KismetMathLibrary.RandomFloatInRangeFromStream` -1000.0 1000.0 _randstream))) "AdjustIfPossibleButDontSpawnIfColliding" "OverrideRootScale"))
    (bind (_origin _boxextent _sphereradius) (`KismetSystemLibrary.GetComponentBounds` (`/Game/Blueprints/OctreeDemoElement.Cube` _returnvalue)))
    (`self.AddOctreeElement` (make `OctreeElement` _returnvalue (`KismetMathLibrary.MakeBoxSphereBounds` _origin _boxextent _sphereradius)))))

(event `self.ReceiveActorBeginOverlap`
  (params (OtherActor :type "Actor Object Reference")))

(event `self.ReceiveTick`
  (params (DeltaSeconds :type "Float (single-precision)")))

(fn `UserConstructionScript`)